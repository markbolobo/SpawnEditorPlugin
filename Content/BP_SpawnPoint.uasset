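; BP_SpawnPoint is a clickable spawn point actor that gives itself an index among the other spawn points in the level.
; When its index is zero, the construction script gathers the positive indices of all spawn points and takes a missing number within their count, otherwise the next one.
; Clicking the actor prints a debug string and fires the EDActorOnClicked dispatcher with its index.
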(event `self.ReceiveActorOnClicked`
  (params (ButtonPressed :type "Key Structure"))
  (`KismetSystemLibrary.PrintString` "Hello")
  (`self.ED_ActorOnClicked` (`self.mIndex`)))

(fn `UserConstructionScript`
  (locals (aTempAllIndex :type "Array of Integer"))
  (bind _returnvalue (`KismetArrayLibrary.Array_Length` (`local.aTempAllIndex`)))
  (if (== (`self.mIndex`) 0)
    (bind _outactors (`GameplayStatics.GetAllActorsOfClass` "BP_SpawnPoint_C"))
    (for _array_element _outactors
      (bind _mindex (`/Game/BP_SpawnPoint.mIndex` _array_element))
      (if (> _mindex 0)
        (`KismetArrayLibrary.Array_AddUnique` (`local.aTempAllIndex`) _mindex)))
    (if (!= _returnvalue 0)
      (for _index (range 1 (+ _returnvalue 1))
        (if (not (`KismetArrayLibrary.Array_Contains` (`local.aTempAllIndex`) _index))
          (set `self.mIndex` _index)))
      (if (== (`self.mIndex`) 0)
        (set `self.mIndex` (+ _returnvalue 1)))
      (else
        (set `self.mIndex` 1)))))